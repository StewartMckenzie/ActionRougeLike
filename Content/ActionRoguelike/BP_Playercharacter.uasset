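; Player character Blueprint for the ActionRoguelike game that sets up the player's HUD and reports health changes.
; On BeginPlay it creates the crosshair and player health widgets and adds both to the viewport.
; The AttributeComp OnHealthChanged event prints the new health on screen as debug output.
; Tick and the construction script are empty, and a second health print is left unconnected.
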(event OnHealthChanged(AttributeComp)
  (params (InstigatorActor :type Actor%20Object%20Reference) (OwningComp :type S%20Attribute%20Component%20Object%20Reference) (NewHealth :type Float%20%28single-precision%29) (Delta :type Float%20%28single-precision%29))
  (Development|PrintString (Utilities|String|ToString(Float) NewHealth) true true "(R=1.000000,G=0.633787,B=0.000000,A=1.000000)"))

(event EventBeginPlay
  (bind _returnvalue (UserInterface|CreateWidget "/Game/ActionRoguelike/UI/UI_CroshairWidget.UI_CroshairWidget_C"))
  (UserInterface|Viewport|AddtoViewport _returnvalue 0)
  (bind _returnvalue_2 (UserInterface|CreateWidget "/Game/ActionRoguelike/UI/UI_PlayerHealth_widget.UI_PlayerHealth_widget_C"))
  (UserInterface|Viewport|AddtoViewport _returnvalue_2 0))

(event Collision|EventActorBeginOverlap
  (params (OtherActor :type Actor%20Object%20Reference)))

(event EventTick
  (params (DeltaSeconds :type Float%20%28single-precision%29)))

(fn ConstructionScript)